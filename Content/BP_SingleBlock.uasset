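; BP_SingleBlock is a block actor that glows in its BlockColor and eases vertically toward a target height.
; On BeginPlay it pushes BlockColor into the GlowColor material parameter of its StaticMesh and sets TargetZ to its starting height.
; Each Tick it lerps Z by a fixed fraction toward TargetZ until nearly equal, giving a frame-rate-dependent ease-out whenever TargetZ differs from its height.
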(event `self.ReceiveBeginPlay`
  (bind (_returnvalue_x _returnvalue_y _returnvalue_z) (`KismetMathLibrary.BreakVector` (`self.K2_GetActorLocation`)))
  (`MeshComponent.SetVectorParameterValueOnMaterials` (`self.StaticMesh`) "GlowColor" (`KismetMathLibrary.Conv_LinearColorToVector` (`self.BlockColor`)))
  (set `self.Target Z` _returnvalue_z))

(event `self.ReceiveTick`
  (params (DeltaSeconds :type "Float (single-precision)"))
  (bind (_returnvalue_x _returnvalue_y _returnvalue_z) (`KismetMathLibrary.BreakVector` (`self.K2_GetActorLocation`)))
  (bind _target_z (`self.Target Z`))
  (if (not (`KismetMathLibrary.NearlyEqual_FloatFloat` _returnvalue_z _target_z 0.01))
    (`self.K2_SetActorLocation` (`KismetMathLibrary.MakeVector` _returnvalue_x _returnvalue_y (`KismetMathLibrary.Lerp` _returnvalue_z _target_z 0.05)))))

(fn `UserConstructionScript`)
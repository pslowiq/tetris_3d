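; BP_GameMode is the game mode, which lays out line detectors and starts the score UI.
; On BeginPlay, nested loops spawn a grid of BP_LineDetector actors at fixed spacing from LineStartingPosition, with LineAmount setting the vertical extent.
; Score reset and BP_UI creation sit inside the inner loop, so a new widget is added to the viewport for every detector spawned.
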(event `self.ReceiveBeginPlay`
  (for _index (range 6)
    (for _index_2 (range (+ (`self.LineAmount`) 1))
      (`|SpawnActorFromClass` "/Game/BP_LineDetector.BP_LineDetector_C" (`KismetMathLibrary.MakeTransform` (+ (`KismetMathLibrary.MakeVector` 0.0 (+ (* _index 50) -100) (* _index_2 50)) (`self.LineStartingPosition`))) "Undefined" "OverrideRootScale" null null)
      (set `self.Score` 0)
      (bind _returnvalue (`|CreateWidget` "/Game/BP_UI.BP_UI_C"))
      (`UserWidget.AddToViewport` _returnvalue 0))))

(fn `UserConstructionScript`)
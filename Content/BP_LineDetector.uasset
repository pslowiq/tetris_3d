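; BP_LineDetector is a line-clear detector for what appears to be a falling-block puzzle game.
; CheckLines, not called within this Blueprint, treats exactly 19 BP_SingleBlock actors overlapping its box as a full line.
; It explodes and destroys them, then adds score to BP_GameMode.
; Blocks at exactly the detector's Y and at or above its height then get their TargetZ lowered one step.
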(event `self.ReceiveBeginPlay`)

(fn `Check Lines`
  (bind (_returnvalue_x _returnvalue_y) (`KismetMathLibrary.BreakVector` (`self.K2_GetActorLocation`)))
  (bind (_returnvalue_x_2 _returnvalue_y_2 _returnvalue_z) (`KismetMathLibrary.BreakVector` (`self.K2_GetActorLocation`)))
  (bind _output_get (set `self.Overlapping Actors` (`PrimitiveComponent.GetOverlappingActors` (`self.GetComponentByClass` "/Script/Engine.BoxComponent") "/Game/BP_SingleBlock.BP_SingleBlock_C")))
  (if (== (`KismetArrayLibrary.Array_Length` _output_get) 19)
    (for _array_element _output_get
      (`GameplayStatics.SpawnEmitterAtLocation` "/Game/StarterContent/Particles/P_Explosion.P_Explosion" (`self.K2_GetActorLocation` _array_element) (struct) (1.5 1.5 1.5))
      (`self.K2_DestroyActor` _array_element))
    (bind _asbp_game_mode (cast `/Game/BP_GameMode` (`GameplayStatics.GetGameMode`)))
    (set `/Game/BP_GameMode.Score` (+ (`/Game/BP_GameMode.Score` _asbp_game_mode) 100) _asbp_game_mode)
    (bind _outactors (`GameplayStatics.GetAllActorsOfClass` "/Game/BP_SingleBlock.BP_SingleBlock_C"))
    (for _array_element_2 _outactors
      (bind (_returnvalue_x_3 _returnvalue_y_3 _returnvalue_z_2) (`KismetMathLibrary.BreakVector` (`self.K2_GetActorLocation` _array_element_2)))
      (if (and (== _returnvalue_y_3 _returnvalue_y) (>= _returnvalue_z_2 _returnvalue_z))
        (set `/Game/BP_SingleBlock.Target Z` (- (`/Game/BP_SingleBlock.Target Z` _array_element_2) 50.0) _array_element_2)))))

(fn `UserConstructionScript`)
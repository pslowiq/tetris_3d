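; Player-controlled falling piece for a 3D Tetris-style game, built from four cubes in a random shape and color at construction.
; A looping timer steps it down until line traces hit, then it becomes BP_SingleBlocks, spawns the next piece and triggers BP_LineDetector checks.
; Input moves and rotates it, undoing changes on box overlap, with directions flipped by BP_Camera's switch.
; Speed-up uses global time dilation.
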(event `InputAction|RotateBlockHorizontal`
  (params (Key :type "Key Structure"))
  (:`Pressed`
    (`self.Rotate Block` (0.0 0.0 90.0))))

(event `InputAction|RotateBlockVertical`
  (params (Key :type "Key Structure"))
  (:`Pressed`
    (`self.Rotate Block` (0.0 90.0 0.0))))

(event `InputAction|SpeedUpBlock`
  (params (Key :type "Key Structure"))
  (:`Pressed`
    (`GameplayStatics.SetGlobalTimeDilation` 5.0))
  (:`Released`
    (`GameplayStatics.SetGlobalTimeDilation` 1.0)))

(event `InputAction|MoveLeft`
  (params (Key :type "Key Structure"))
  (:`Pressed`
    (if (`self.Get Camera Switch`)
      (`self.BlockMovement` (50.0 0.0 0.0) :!label _label)
      (else
        (`self.BlockMovement` (-50.0 0.0 0.0) :!label _label_2)))))

(event `InputAction|MoveRight`
  (params (Key :type "Key Structure"))
  (:`Pressed`
    (if (`self.Get Camera Switch`)
      (goto _label_2)
      (else
        (goto _label)))))

(event `InputAction|MoveForward`
  (params (Key :type "Key Structure"))
  (:`Pressed`
    (if (`self.Get Camera Switch`)
      (`self.BlockMovement` (0.0 50.0 0.0) :!label _label_3)
      (else
        (`self.BlockMovement` (0.0 -50.0 0.0) :!label _label_4)))))

(event `InputAction|MoveBackward`
  (params (Key :type "Key Structure"))
  (:`Pressed`
    (if (`self.Get Camera Switch`)
      (goto _label_4)
      (else
        (goto _label_3)))))

(event `self.ReceiveBeginPlay`
  (bind _returnvalue (`KismetSystemLibrary.K2_SetTimerDelegate` (delegate `DropBlock`) (`self.Falling Interval`) true))
  (set `self.Block Timer` _returnvalue))

(event `DropBlock`
  (set `self.IsFalling` true)
  (for _array_element (`SceneComponent.GetChildrenComponents` (`self.DefaultSceneRoot`) false)
    (bind _returnvalue (`SceneComponent.K2_GetComponentLocation` _array_element))
    (bind (_outhit _returnvalue_2) (`KismetSystemLibrary.LineTraceSingleForObjects` _returnvalue (- _returnvalue (0.0 0.0 50.0)) (`|MakeArray` "ObjectTypeQuery1" :!type "EObjectTypeQuery Enum")))
    (if _returnvalue_2
      (`/Engine/EditorBlueprintResources/StandardMacros.DoOnce` false
        (:`Completed`
          (set `self.IsFalling` false)
          (`KismetSystemLibrary.K2_ClearAndInvalidateTimerHandle` (`self.Block Timer`))))))
  (if (`self.IsFalling`)
    (`self.K2_AddActorWorldOffset` (0.0 0.0 -50.0))
    (else
      (for _array_element_2 (`SceneComponent.GetChildrenComponents` (`self.DefaultSceneRoot`) false)
        (`|SpawnActorFromClass` "/Game/BP_SingleBlock.BP_SingleBlock_C" (`KismetMathLibrary.MakeTransform` (`SceneComponent.K2_GetComponentLocation` _array_element_2)) "Undefined" "OverrideRootScale" null (`self.BlockColor`) null))
      (`self.K2_DestroyActor`)
      (`|SpawnActorFromClass` "BP_FallingBlock_C" (`KismetMathLibrary.MakeTransform` (0.0 0.0 1050.0)) "Undefined" "OverrideRootScale" null null)
      (bind _outactors (`GameplayStatics.GetAllActorsOfClass` "/Game/BP_LineDetector.BP_LineDetector_C"))
      (for _array_element_3 _outactors
        (`/Game/BP_LineDetector.Check Lines` _array_element_3)))))

(fn `BlockMovement`
  (params (Amount :type "Vector Structure"))
  (`self.K2_AddActorWorldOffset` Amount)
  (for _array_element (`self.K2_GetComponentsByClass` "/Script/Engine.StaticMeshComponent")
    (bind (_outactors _returnvalue) (`KismetSystemLibrary.BoxOverlapActors` (`SceneComponent.K2_GetComponentLocation` _array_element) (15.0 15.0 15.0) (`|MakeArray` "ObjectTypeQuery1" :!type "EObjectTypeQuery Enum")))
    (if _returnvalue
      (`self.K2_AddActorWorldOffset` (* Amount -1.0))
      (break))))

(fn `Get Camera Switch`
  (returns (IsSwitched :type Boolean))
  (bind _asbp_camera (cast `/Game/BP_Camera` (`GameplayStatics.GetPlayerPawn` 0)))
  (return (`/Game/BP_Camera.IsSwitched` _asbp_camera)))

(fn `Rotate Block`
  (params (Rotation :type "Vector Structure"))
  (`self.K2_AddActorLocalRotation` (`KismetMathLibrary.Conv_VectorToRotator` Rotation))
  (for _array_element (`self.K2_GetComponentsByClass` "/Script/Engine.StaticMeshComponent")
    (bind (_outactors _returnvalue) (`KismetSystemLibrary.BoxOverlapActors` (`SceneComponent.K2_GetComponentLocation` _array_element) (15.0 15.0 15.0) (`|MakeArray` "ObjectTypeQuery1" :!type "EObjectTypeQuery Enum")))
    (if _returnvalue
      (`self.K2_AddActorLocalRotation` (`KismetMathLibrary.Conv_VectorToRotator` (* Rotation -1.0)))
      (break))))

(fn `UserConstructionScript`
  (switch `int` (`KismetMathLibrary.RandomIntegerInRange` 0 3)
    (:`0`
      ;[1 1 1] Line block
      (`SceneComponent.K2_AddLocalOffset` (`self.Cube2`) (0.0 0.0 50.0) false false)
      (`SceneComponent.K2_AddLocalOffset` (`self.Cube3`) (0.0 0.0 100.0) false false)
      (`SceneComponent.K2_AddLocalOffset` (`self.Cube4`) (0.0 0.0 150.0) false false)
      (set `self.BlockColor` (struct :`R` 1.0 :`G` 0.128853 :`B` 0.838526 :`A` 1.0))
      (`MeshComponent.SetVectorParameterValueOnMaterials` (`self.Cube1`) "GlowColor" (`KismetMathLibrary.Conv_LinearColorToVector` (`self.BlockColor`)) :!label _label)
      (`MeshComponent.SetVectorParameterValueOnMaterials` (`self.Cube2`) "GlowColor" (`KismetMathLibrary.Conv_LinearColorToVector` (`self.BlockColor`)))
      (`MeshComponent.SetVectorParameterValueOnMaterials` (`self.Cube3`) "GlowColor" (`KismetMathLibrary.Conv_LinearColorToVector` (`self.BlockColor`)))
      (`MeshComponent.SetVectorParameterValueOnMaterials` (`self.Cube4`) "GlowColor" (`KismetMathLibrary.Conv_LinearColorToVector` (`self.BlockColor`))))
    (:`1`
      ;[1 1 1] T block
      (`SceneComponent.K2_AddLocalOffset` (`self.Cube2`) (50.0 0.0 0.0) false false)
      (`SceneComponent.K2_AddLocalOffset` (`self.Cube3`) (-50.0 0.0 0.0) false false)
      (`SceneComponent.K2_AddLocalOffset` (`self.Cube4`) (50.0 0.0 50.0) false false)
      (set `self.BlockColor` (struct :`G` 1.0 :`B` 0.168349 :`A` 1.0))
      (goto _label))
    (:`2`
      ;[1 1 1] Cube block
      (`SceneComponent.K2_AddLocalOffset` (`self.Cube2`) (50.0 0.0 0.0) false false)
      (`SceneComponent.K2_AddLocalOffset` (`self.Cube3`) (0.0 0.0 50.0) false false)
      (`SceneComponent.K2_AddLocalOffset` (`self.Cube4`) (50.0 0.0 50.0) false false)
      (set `self.BlockColor` (struct :`R` 1.0 :`B` 0.095176 :`A` 1.0))
      (goto _label))
    (:`3`
      ;[1 1 1] L block
      (`SceneComponent.K2_AddLocalOffset` (`self.Cube2`) (0.0 0.0 50.0) false false)
      (`SceneComponent.K2_AddLocalOffset` (`self.Cube3`) (0.0 0.0 100.0) false false)
      (`SceneComponent.K2_AddLocalOffset` (`self.Cube4`) (50.0 0.0 100.0) false false)
      (set `self.BlockColor` (struct :`R` 1.0 :`G` 0.898209 :`A` 1.0)))))